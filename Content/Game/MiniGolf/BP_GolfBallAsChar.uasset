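; Mini-golf ball implemented as a Character, aimed with mouse look and launched along the camera's horizontal yaw.
; Holding left mouse builds LaunchSpeed on Tick without a cap and prints it; releasing resets it to zero.
; Space calls LaunchCharacter with that speed, so it only has force while the button is held.
; CanLaunch gates the shot on near-zero velocity, but updates only while charging.
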(event `self.ReceiveTick`
  (params (DeltaSeconds :type "Float (single-precision)"))
  (if (`self.isCharging`)
    (bind _output_get (set `self.LaunchSpeed` (+ (* DeltaSeconds 1500.0) (`self.LaunchSpeed`))))
    (`KismetSystemLibrary.PrintString` (`KismetStringLibrary.Conv_DoubleToString` _output_get))
    (if (<= (`KismetMathLibrary.VSize` (`self.GetVelocity`)) 0.1)
      (set `self.canLaunch` true)
      (else
        (set `self.canLaunch` false)))))

(event `Key|LeftMouseButton`
  (params (Key :type "Key Structure"))
  (:`Pressed`
    (set `self.isCharging` true))
  (:`Released`
    (set `self.isCharging` false)
    (set `self.LaunchSpeed` 0.0)))

(event `InputAxis|Turn Right / Left Mouse`
  (params (AxisValue :type "Float (single-precision)"))
  ;[1 1 1] Camera Inputs
  (`self.AddControllerYawInput` AxisValue))

(event `Key|SpaceBar`
  (params (Key :type "Key Structure"))
  (:`Pressed`
    (if (`self.canLaunch`)
      (`self.LaunchCharacter` (* (`KismetMathLibrary.GetForwardVector` (`KismetMathLibrary.MakeRotator` 0.0 0.0 (.yaw (`self.GetControlRotation`)))) (`self.LaunchSpeed`))))))

(event `InputAxis|Look Up / Down Mouse`
  (params (AxisValue :type "Float (single-precision)"))
  ;[1 1 1] Camera Inputs
  (`self.AddControllerPitchInput` AxisValue))

(fn `UserConstructionScript`)