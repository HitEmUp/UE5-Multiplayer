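; BP_CoopDoor is a co-op door that opens while both trigger boxes, BoxL and BoxR, hold a third-person character.
; Any begin or end overlap on either box makes the authority re-check both boxes through CheckOverlapping.
; OpenCloseDoor then snaps the Door to a fixed open or closed world rotation, alongside a debug print.
; The check takes the first overlapping character in each box without confirming they are different players.
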(event `OpenCloseDoor`
  (params (`OpenIt?` :type Boolean))
  (bind _door (`self.Door`))
  (if `OpenIt?`
    (`SceneComponent.K2_SetWorldRotation` _door (struct :`Yaw` 90.0) false false)
    (else
      (`SceneComponent.K2_SetWorldRotation` _door (struct) false false))))

(event `CheckOverlapping`
  (cast `/Game/ThirdPerson/Blueprints/BP_ThirdPersonCharacter` (`|GetArrayItem` (`PrimitiveComponent.GetOverlappingActors` (`self.BoxL`) "/Game/ThirdPerson/Blueprints/BP_ThirdPersonCharacter.BP_ThirdPersonCharacter_C"))
    (:`then`
      (cast `/Game/ThirdPerson/Blueprints/BP_ThirdPersonCharacter` (`|GetArrayItem` (`PrimitiveComponent.GetOverlappingActors` (`self.BoxR`) "/Game/ThirdPerson/Blueprints/BP_ThirdPersonCharacter.BP_ThirdPersonCharacter_C"))
        (:`then`
          (`self.OpenCloseDoor` true)
          (`KismetSystemLibrary.PrintString` "OpenDoor" true true (struct :`R` 0.164896 :`G` 1.0 :`A` 1.0) 5.0))
        (:`CastFailed`
          (`self.OpenCloseDoor` false :!label _label)
          (`KismetSystemLibrary.PrintString` "CloseDoor" true true (struct :`R` 1.0 :`B` 0.068537 :`A` 1.0) 5.0))))
    (:`CastFailed`
      (goto _label))))

(event `self.BoxL.OnComponentEndOverlap`
  (params (OverlappedComponent :type "PrimitiveComponent Object Reference") (OtherActor :type "Actor Object Reference") (OtherComp :type "PrimitiveComponent Object Reference") (OtherBodyIndex :type Integer))
  (`/Engine/EditorBlueprintResources/ActorMacros.Switch Has Authority` :!label _label_2
    (:`Authority`
      (`self.CheckOverlapping`))))

(event `self.BoxL.OnComponentBeginOverlap`
  (params (OverlappedComponent :type "PrimitiveComponent Object Reference") (OtherActor :type "Actor Object Reference") (OtherComp :type "PrimitiveComponent Object Reference") (OtherBodyIndex :type Integer) (bFromSweep :type Boolean) (SweepResult :type "HitResult Structure (by ref)"))
  (goto _label_2))

(event `self.BoxR.OnComponentBeginOverlap`
  (params (OverlappedComponent :type "PrimitiveComponent Object Reference") (OtherActor :type "Actor Object Reference") (OtherComp :type "PrimitiveComponent Object Reference") (OtherBodyIndex :type Integer) (bFromSweep :type Boolean) (SweepResult :type "HitResult Structure (by ref)"))
  (goto _label_2))

(event `self.BoxR.OnComponentEndOverlap`
  (params (OverlappedComponent :type "PrimitiveComponent Object Reference") (OtherActor :type "Actor Object Reference") (OtherComp :type "PrimitiveComponent Object Reference") (OtherBodyIndex :type Integer))
  (goto _label_2))

(fn `UserConstructionScript`)