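; Lobby player controller that gives each player a lobby widget with chat and a player list.
; On BeginPlay it shows WBP_Lobby in UI-only input and sends the GameInstance nickname through ServerSetNickname.
; Server events store status or format nickname-prefixed messages, then have BP_GameModeLobby update or broadcast to clients.
; AddMessage and ClientUpdatePlayerlist pass incoming data to the widget; a nickname debug timer is left disconnected.
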(event `self.ReceiveBeginPlay`
  ;[1 1 1] beginplay und init stuff
  (bind _returnvalue (`|CreateWidget` "/Game/Blueprints/UI/WBP_Lobby.WBP_Lobby_C" (`GameplayStatics.GetPlayerController` 0)))
  (bind _output_get (set `self.WBPChat` _returnvalue))
  (`UserWidget.AddToViewport` _output_get 0)
  (`WidgetBlueprintLibrary.SetInputMode_UIOnlyEx` self _output_get)
  (set `self.bShowMouseCursor` true)
  (`self.GetAndSafeNicknameFromGI`))

(event `TesteLokalNickname`
  ;[1 1 1] Test bzgl. nickname
  (`KismetSystemLibrary.PrintString` (`KismetStringLibrary.Concat_StrStr` "Client say my Nickname is:" (`self.Nickname`))))

(event `GetAndSafeNicknameFromGI`
  ;[1 1 1] Nickname Updates
  (bind _asbp_my_game_instance (cast `/Game/Game/BP_MyGameInstance` (`GameplayStatics.GetGameInstance`)))
  (`self.ServerSetNickname` (`/Game/Game/BP_MyGameInstance.LocalNickname` _asbp_my_game_instance)))

(event `ServerSetMyPlayerStatus`
  (params (PlayerStatus :type "/Game/Blueprints/S_PlayerStatus Structure"))
  ;[1 1 1] Playerlisten updates
  (set `self.PlayerStatus` PlayerStatus)
  (bind _asbp_game_mode_lobby (cast `/Game/Game/BP_GameModeLobby` (`GameplayStatics.GetGameMode`)))
  (`/Game/Game/BP_GameModeLobby.SendUpdateUIToClients` _asbp_game_mode_lobby))

(event `ServerSetNickname`
  (params (Nickname :type String))
  ;[1 1 1] Nickname Updates
  (set `self.Nickname` Nickname))

(event `ClientUpdatePlayerlist`
  (params (PlayerStatus :type "Array of /Game/Blueprints/S_PlayerStatus Structure (by ref)"))
  ;[1 1 1] Playerlisten updates
  (`/Game/Blueprints/UI/WBP_Lobby.RefreshPlayerlist` (`self.WBPChat`) PlayerStatus))

(event `ServerSendMessage`
  (params (Message :type Text))
  ;[1 1 1] Chat
  (bind _asbp_game_mode_lobby (cast `/Game/Game/BP_GameModeLobby` (`GameplayStatics.GetGameMode`)))
  (`/Game/Game/BP_GameModeLobby.SendMessageToAll` _asbp_game_mode_lobby (`|FormatText` "{0}: {1}" (`self.Nickname`) Message)))

(event `AddMessage`
  (params (Message :type Text))
  ;[1 1 1] Chat
  (`/Game/Blueprints/UI/WBP_Lobby.AddMessageToScrollbox` (`self.WBPChat`) Message))

(fn `UserConstructionScript`)