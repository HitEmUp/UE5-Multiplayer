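; BP_GMGame is a game mode Blueprint that handles death and respawn for players controlling BP_ThirdPersonCharacter.
; It collects player controllers in the PCs array through OnSwapPlayerControllers.
; Its server-only CheackHealth event loops over them, destroys any character at or below zero Health, then spawns and possesses a replacement.
; The loop stops at the first controller whose pawn fails the cast.
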(event `self.K2_OnSwapPlayerControllers`
  (params (OldPC :type "PlayerController Object Reference") (NewPC :type "PlayerController Object Reference"))
  (`KismetArrayLibrary.Array_AddUnique` (`self.PCs`) NewPC))

(event `CheackHealth`
  (`/Engine/EditorBlueprintResources/ActorMacros.Switch Has Authority`
    (:`Authority`
      (if (`KismetSystemLibrary.IsServer`)
        (for _array_element (`self.PCs`)
          (bind _asbp_third_person_character (cast `/Game/ThirdPerson/Blueprints/BP_ThirdPersonCharacter` (`Controller.K2_GetPawn` _array_element)))
          (if (<= (`/Game/ThirdPerson/Blueprints/BP_ThirdPersonCharacter.Health` _asbp_third_person_character) 0.0)
            (`self.K2_DestroyActor` _asbp_third_person_character)
            (bind _returnvalue (`|SpawnActorFromClass` "/Game/ThirdPerson/Blueprints/BP_ThirdPersonCharacter.BP_ThirdPersonCharacter_C" (`KismetMathLibrary.MakeTransform` (0.0 0.0 0.0)) "Undefined" "MultiplyWithRoot" null null))
            (`Controller.Possess` _array_element _returnvalue)))))))

(fn `UserConstructionScript`)