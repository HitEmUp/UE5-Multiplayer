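; BP_FPSShooterCharacter is a shooter character Blueprint that fires a hitscan shot on the Fire input.
; FireOnServer runs only with authority, line-tracing from the muzzle socket along the skeletal mesh's right vector with debug drawing.
; A blocking hit prints the actor's name and calls MuzzleHitVFX, which spawns asphalt impact Niagara effects for world objects or blood for pawns.
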(event `InputAction|Fire`
  (params (Key :type "Key Structure"))
  (:`Pressed`
    (`self.FireOnServer`)))

(event `FireOnServer`
  (bind _skeletalmesh (`self.SkeletalMesh`))
  (bind _returnvalue (`SceneComponent.GetSocketLocation` _skeletalmesh "muzzleSocket"))
  (`/Engine/EditorBlueprintResources/ActorMacros.Switch Has Authority`
    (:`Authority`
      (bind _outhit (`KismetSystemLibrary.LineTraceSingleForObjects` :`Start` _returnvalue :`End` (+ _returnvalue (* (`SceneComponent.GetRightVector` _skeletalmesh) 1000.0)) :`ObjectTypes` (`self.Object Types`) :`DrawDebugType` "ForDuration"))
      (if (`GameplayStatics.BreakHitResult` _outhit)
        (`KismetSystemLibrary.PrintString` (`KismetSystemLibrary.GetDisplayName` (`.HitActor` (`GameplayStatics.BreakHitResult` _outhit))))
        (`self.MuzzleHitVFX` (`.ImpactPoint` (`GameplayStatics.BreakHitResult` _outhit)) (`PrimitiveComponent.GetCollisionObjectType` (`.HitComponent` (`GameplayStatics.BreakHitResult` _outhit))))))))

(event `MuzzleHitVFX`
  (params (Location :type "Vector Structure") (NewParam2 :type "ECollisionChannel Enum" :default "ECC_WorldStatic"))
  (switch `ECollisionChannel` NewParam2
    (:`ECC_WorldStatic`
      (`NiagaraFunctionLibrary.SpawnSystemAtLocation` "/Game/ImpactsVFXVol1/Niagara/NS_ImpactAsphalt.NS_ImpactAsphalt" Location :!label _label))
    (:`ECC_WorldDynamic`
      (goto _label))
    (:`ECC_Pawn`
      (`NiagaraFunctionLibrary.SpawnSystemAtLocation` "/Game/ImpactsVFXVol1/Niagara/NS_ImpactBlood.NS_ImpactBlood" Location))))

(fn `UserConstructionScript`)