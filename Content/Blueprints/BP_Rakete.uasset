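; BP_Rakete is a rocket projectile actor that damages player characters on contact and credits the shooter.
; On authority, its box overlap removes health from a hit BP_MyTPCharacter and spawns an explosion particle at the mesh location.
; The instigator's BP_PlayerStateFLevel gains a hit, plus a kill when the victim's health is depleted, then the rocket destroys itself after a short delay.
; Overlaps with other actor types are ignored.
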(event `self.Box.OnComponentBeginOverlap`
  (params (OverlappedComponent :type "PrimitiveComponent Object Reference") (OtherActor :type "Actor Object Reference") (OtherComp :type "PrimitiveComponent Object Reference") (OtherBodyIndex :type Integer) (bFromSweep :type Boolean) (SweepResult :type "HitResult Structure (by ref)"))
  (`/Engine/EditorBlueprintResources/ActorMacros.Switch Has Authority`
    (:`Authority`
      (bind _asbp_my_tpcharacter (cast `/Game/Blueprints/BP_MyTPCharacter` OtherActor))
      (`/Game/Blueprints/BP_MyTPCharacter.AddHealth` _asbp_my_tpcharacter -10.0)
      (`self.SpawnEmitter`)
      (bind _asbp_player_state_flevel (cast `/Game/Game/FirstLevel/BP_PlayerStateFLevel` (`Controller.PlayerState` (`self.GetInstigatorController`))))
      (if (<= (`/Game/Blueprints/BP_MyTPCharacter.Health` _asbp_my_tpcharacter) 0.0)
        (`/Game/Game/FirstLevel/BP_PlayerStateFLevel.AddHits` _asbp_player_state_flevel)
        (`/Game/Game/FirstLevel/BP_PlayerStateFLevel.AddKills` _asbp_player_state_flevel)
        (else
          (`/Game/Game/FirstLevel/BP_PlayerStateFLevel.AddHits` _asbp_player_state_flevel)))
      (`KismetSystemLibrary.Delay` 0.2)
      (`self.K2_DestroyActor`))))

(event `SpawnEmitter`
  (`GameplayStatics.SpawnEmitterAtLocation` "/Game/StarterContent/Particles/P_Explosion.P_Explosion" (`SceneComponent.K2_GetComponentLocation` (`self.StaticMesh`))))

(fn `UserConstructionScript`)