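; Manager actor for a cube puzzle that checks whether the puzzle is solved and shows the result on a spotlight.
; CheckPuzzle runs only with authority and loops over every BP_CubePuzzle, setting PuzzleDone false and stopping at the first cube not hitting another.
; It then prints the state and calls MulticastLight to turn the light green when done or red otherwise.
; The solved branch has only a placeholder message, with no further gameplay effect.
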(event `CheckPuzzle`
  (`/Engine/EditorBlueprintResources/ActorMacros.Switch Has Authority`
    (:`Authority`
      (bind _outactors (`GameplayStatics.GetAllActorsOfClass` "/Game/Blueprints/BP_CubePuzzle.BP_CubePuzzle_C"))
      (for _array_element _outactors
        (if (`/Game/Blueprints/BP_CubePuzzle.IsHittingOtherCube` _array_element)
          (set `self.Puzzle Done` true)
          (else
            (set `self.Puzzle Done` false)
            (break))))
      (if (`self.Puzzle Done`)
        (`KismetSystemLibrary.PrintString` "Puzzle done, do something!" true true (struct :`R` 0.342295 :`G` 1.0 :`A` 1.0))
        (`self.MulticastLight` (struct :`R` 0.012644 :`G` 1.0 :`A` 1.0))
        (else
          (`KismetSystemLibrary.PrintString` "Puzzle is not done!" true true (struct :`R` 1.0 :`G` 0.093707 :`A` 1.0))
          (`self.MulticastLight` (struct :`R` 1.0 :`A` 1.0)))))))

(event `MulticastLight`
  (params (NewLightColor :type "LinearColor Structure"))
  (`LightComponent.SetLightColor` (`self.SpotLight`) NewLightColor true))

(fn `UserConstructionScript`)