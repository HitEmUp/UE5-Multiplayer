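; BP_CubePuzzle is a networked puzzle cube that rotates a 45-degree step when something overlaps its Sphere, once until an overlap ends.
; After rotating, the server line-traces along the cube's forward vector to set whether it hits another puzzle cube, then has BP_CubePuzzleManager check the puzzle.
; The RepNotify on that flag turns the cube green while it hits another cube.
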(event `self.Sphere.OnComponentBeginOverlap`
  (params (OverlappedComponent :type "PrimitiveComponent Object Reference") (OtherActor :type "Actor Object Reference") (OtherComp :type "PrimitiveComponent Object Reference") (OtherBodyIndex :type Integer) (bFromSweep :type Boolean) (SweepResult :type "HitResult Structure (by ref)"))
  (`/Engine/EditorBlueprintResources/ActorMacros.Switch Has Authority`
    (:`Authority`
      (`/Engine/EditorBlueprintResources/StandardMacros.DoOnce` false :!label _label
        (:`Completed`
          (`self.K2_AddActorWorldRotation` (struct :`Yaw` 45.0))
          (`self.CheckIsHitting`))))))

(event `self.Sphere.OnComponentEndOverlap`
  (params (OverlappedComponent :type "PrimitiveComponent Object Reference") (OtherActor :type "Actor Object Reference") (OtherComp :type "PrimitiveComponent Object Reference") (OtherBodyIndex :type Integer))
  (`/Engine/EditorBlueprintResources/ActorMacros.Switch Has Authority`
    (:`Authority`
      (goto _label :!via `Reset`))))

(event `CheckIsHitting`
  (bind _returnvalue (`self.K2_GetActorLocation`))
  (`/Engine/EditorBlueprintResources/ActorMacros.Switch Has Authority`
    (:`Authority`
      (bind _outhit (`KismetSystemLibrary.LineTraceSingle` :`Start` _returnvalue :`End` (+ _returnvalue (* (`self.GetActorForwardVector`) 5000.0)) :`TraceChannel` "TraceTypeQuery1" :`DrawDebugType` "ForOneFrame"))
      (cast `/Game/Blueprints/BP_CubePuzzle` (`.HitActor` (`GameplayStatics.BreakHitResult` _outhit))
        (:`then`
          (set `self.IsHittingOtherCube` true))
        (:`CastFailed`
          (set `self.IsHittingOtherCube` false)))
      (bind _outactors (`GameplayStatics.GetAllActorsOfClass` "/Game/Blueprints/BP_CubePuzzleManager.BP_CubePuzzleManager_C"))
      (`/Game/Blueprints/BP_CubePuzzleManager.CheckPuzzle` (`|GetArrayItem` _outactors)))))

(fn `OnRep_IsHittingOtherCube`
  (bind _cube (`self.Cube`))
  (if (`self.IsHittingOtherCube`)
    (`PrimitiveComponent.SetMaterial` _cube 0 "/AnimationSharing/AnimSharingGreen.AnimSharingGreen")
    (else
      (`PrimitiveComponent.SetMaterial` _cube 0 "/Engine/BasicShapes/BasicShapeMaterial.BasicShapeMaterial"))))

(fn `UserConstructionScript`)