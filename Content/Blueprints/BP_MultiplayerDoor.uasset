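; A co-op door Blueprint that opens only while player pawns 0 and 1 each stand in a separate trigger box, in either order.
; Overlap changes on both boxes feed one authority-only check, which calls open or close.
; A Timeline lerps the door from its start position to a marker component and reverses to close.
; MultiplayerSetLight turns both point lights green when opening and red when closing.
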(event `self.ReceiveBeginPlay`
  (set `self.StartDoorLocation` (`SceneComponent.K2_GetComponentLocation` (`self.Door`))))

(event `DoorOpen`
  (`self.MultiplayerSetLight` (struct :`R` 0.355364 :`G` 1.0 :`A` 1.0))
  (bind (_direction _alpha) (`Timeline|Timeline` :!label _label)
    (:`Update`
      (`SceneComponent.K2_SetWorldLocation` (`self.Door`) (`KismetMathLibrary.VLerp` (`self.StartDoorLocation`) (`SceneComponent.K2_GetComponentLocation` (`self.DoorFinalLocation`)) _alpha) false false))))

(event `MultiplayerSetLight`
  (params (NewLightColor :type "LinearColor Structure"))
  (`LightComponent.SetLightColor` (`self.PointLight`) NewLightColor true)
  (`LightComponent.SetLightColor` (`self.PointLight1`) NewLightColor true))

(event `CloseDoor`
  (`self.MultiplayerSetLight` (struct :`R` 1.0 :`A` 1.0))
  (goto _label :!via `Reverse`))

(event `self.BoxL.OnComponentBeginOverlap`
  (params (OverlappedComponent :type "PrimitiveComponent Object Reference") (OtherActor :type "Actor Object Reference") (OtherComp :type "PrimitiveComponent Object Reference") (OtherBodyIndex :type Integer) (bFromSweep :type Boolean) (SweepResult :type "HitResult Structure (by ref)"))
  (`/Engine/EditorBlueprintResources/ActorMacros.Switch Has Authority` :!label _label_2
    (:`Authority`
      (if (or (and (`PrimitiveComponent.IsOverlappingActor` (`self.BoxL`) (`GameplayStatics.GetPlayerPawn` 0)) (`PrimitiveComponent.IsOverlappingActor` (`self.BoxR`) (`GameplayStatics.GetPlayerPawn` 1))) (and (`PrimitiveComponent.IsOverlappingActor` (`self.BoxL`) (`GameplayStatics.GetPlayerPawn` 1)) (`PrimitiveComponent.IsOverlappingActor` (`self.BoxR`) (`GameplayStatics.GetPlayerPawn` 0))))
        (`self.DoorOpen`)
        (`KismetSystemLibrary.PrintString` "Door Open")
        (else
          (`self.CloseDoor`)
          (`KismetSystemLibrary.PrintString` "Door Open False" true true (struct :`R` 1.0 :`B` 0.050746 :`A` 1.0)))))))

(event `self.BoxL.OnComponentEndOverlap`
  (params (OverlappedComponent :type "PrimitiveComponent Object Reference") (OtherActor :type "Actor Object Reference") (OtherComp :type "PrimitiveComponent Object Reference") (OtherBodyIndex :type Integer))
  (goto _label_2))

(event `self.BoxR.OnComponentBeginOverlap`
  (params (OverlappedComponent :type "PrimitiveComponent Object Reference") (OtherActor :type "Actor Object Reference") (OtherComp :type "PrimitiveComponent Object Reference") (OtherBodyIndex :type Integer) (bFromSweep :type Boolean) (SweepResult :type "HitResult Structure (by ref)"))
  (goto _label_2))

(event `self.BoxR.OnComponentEndOverlap`
  (params (OverlappedComponent :type "PrimitiveComponent Object Reference") (OtherActor :type "Actor Object Reference") (OtherComp :type "PrimitiveComponent Object Reference") (OtherBodyIndex :type Integer))
  (goto _label_2))

(fn `UserConstructionScript`)