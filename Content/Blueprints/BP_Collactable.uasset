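; A networked collectable that holds a random value from 0 to 2, with a matching cone, sphere or box mesh.
; The server rolls the value at BeginPlay, though a second independent roll then overrides the mesh.
; On overlap, the server adds the value to the third-person character and its PlayerState, hides the mesh, then shows and rerolls it after a delay.
; Value's OnRep updates the text render.
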(event `GenerateValue`
  (bind _staticmesh (`self.StaticMesh`))
  (bind _output_get (set `self.Value` (`KismetMathLibrary.RandomIntegerInRange` 0 2)))
  (`KismetSystemLibrary.PrintString` (`KismetStringLibrary.Concat_StrStr` "Value: " (`KismetStringLibrary.Conv_IntToString` _output_get)) true true (struct :`G` 0.66 :`B` 1.0 :`A` 1.0) 120.0 "value")
  (switch `int` _output_get
    (:`Default`
      (`StaticMeshComponent.SetStaticMesh` _staticmesh "/Engine/BasicShapes/Cone.Cone" :!label _label))
    (:`0`
      (goto _label))
    (:`1`
      (`StaticMeshComponent.SetStaticMesh` _staticmesh "/Engine/EditorMeshes/ArcadeEditorSphere.ArcadeEditorSphere"))
    (:`2`
      (`StaticMeshComponent.SetStaticMesh` _staticmesh "/ControlRig/Controls/ControlRig_Box_solid.ControlRig_Box_solid"))))

(event `self.ReceiveBeginPlay`
  (bind _staticmesh (`self.StaticMesh`))
  (`/Engine/EditorBlueprintResources/ActorMacros.Switch Has Authority`
    (:`Authority`
      (`self.GenerateValue`)
      (switch `int` (`KismetMathLibrary.RandomIntegerInRange` 0 2)
        (:`Default`
          (`StaticMeshComponent.SetStaticMesh` _staticmesh "/Engine/BasicShapes/Cone.Cone" :!label _label_2))
        (:`0`
          (goto _label_2))
        (:`1`
          (`StaticMeshComponent.SetStaticMesh` _staticmesh "/Engine/EditorMeshes/ArcadeEditorSphere.ArcadeEditorSphere"))
        (:`2`
          (`StaticMeshComponent.SetStaticMesh` _staticmesh "/ControlRig/Controls/ControlRig_Box_solid.ControlRig_Box_solid"))))))

(event `self.Box.OnComponentBeginOverlap`
  (params (OverlappedComponent :type "PrimitiveComponent Object Reference") (OtherActor :type "Actor Object Reference") (OtherComp :type "PrimitiveComponent Object Reference") (OtherBodyIndex :type Integer) (bFromSweep :type Boolean) (SweepResult :type "HitResult Structure (by ref)"))
  (bind _staticmesh (`self.StaticMesh`))
  (`/Engine/EditorBlueprintResources/ActorMacros.Switch Has Authority`
    (:`Authority`
      (if (`SceneComponent.IsVisible` (`self.StaticMesh`))
        (bind _asbp_third_person_character (cast `/Game/ThirdPerson/Blueprints/BP_ThirdPersonCharacter` OtherActor))
        (`/Game/ThirdPerson/Blueprints/BP_ThirdPersonCharacter.AddValue` _asbp_third_person_character (`KismetMathLibrary.Conv_IntToDouble` (`self.Value`)))
        (bind _asbp_player_stat_game (cast `/Game/Game/BP_PlayerStatGame` (`Pawn.PlayerState` _asbp_third_person_character)))
        (`/Game/Game/BP_PlayerStatGame.AddValue` _asbp_player_stat_game (`self.Value`))
        (`SceneComponent.SetVisibility` _staticmesh false false)
        (`KismetSystemLibrary.Delay` 3.0)
        (`SceneComponent.SetVisibility` _staticmesh true false)
        (`self.GenerateValue`)))))

(fn `OnRep_Value`
  (`TextRenderComponent.K2_SetText` (`self.TextRender`) (`KismetTextLibrary.Conv_IntToText` (`self.Value`)))
  (`KismetSystemLibrary.PrintString` "Wer hat sich geändert"))

(fn `UserConstructionScript`)