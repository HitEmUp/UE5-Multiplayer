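; BP_PlayerControllerChat is a player controller that connects the WBP_Chat chat widget to the game mode.
; On BeginPlay it creates the widget for player controller 0, adds it to the viewport and switches to UI-only input with a visible cursor.
; ServerSendMessage passes text to BP_GameModeChat's SendMessageToAll, while AddMessage appends incoming text to the widget's scrollbox.
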(event `self.ReceiveBeginPlay`
  (bind _returnvalue (`|CreateWidget` "/Game/Blueprints/WBP_Chat.WBP_Chat_C" (`GameplayStatics.GetPlayerController` 0)))
  (bind _output_get (set `self.WBPChat` _returnvalue))
  (`UserWidget.AddToViewport` _output_get 0)
  (`WidgetBlueprintLibrary.SetInputMode_UIOnlyEx` self _output_get)
  (set `self.bShowMouseCursor` true))

(event `ServerSendMessage`
  (params (Message :type Text))
  (bind _asbp_game_mode_chat (cast `/Game/Blueprints/BP_GameModeChat` (`GameplayStatics.GetGameMode`)))
  (`/Game/Blueprints/BP_GameModeChat.SendMessageToAll` _asbp_game_mode_chat Message))

(event `AddMessage`
  (params (Message :type Text))
  (`/Game/Blueprints/WBP_Chat.AddMessageToScrollbox` (`self.WBPChat`) Message))

(fn `UserConstructionScript`)