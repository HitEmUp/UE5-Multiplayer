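; Mini golf map generator that builds an L-shaped course of instanced mesh tiles from length, width and mesh size values.
; The construction script lays one row along X, with a nested loop that re-adds the same Y row on every length step.
; It puts StartLocation at the Y end and the Loch hole at the X end, passing actor-offset positions as relative locations.
; Overlapping the hole only prints the other actor's name with "Finished".
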(event `self.Loch.OnComponentBeginOverlap`
  (params (OverlappedComponent :type "PrimitiveComponent Object Reference") (OtherActor :type "Actor Object Reference") (OtherComp :type "PrimitiveComponent Object Reference") (OtherBodyIndex :type Integer) (bFromSweep :type Boolean) (SweepResult :type "HitResult Structure (by ref)"))
  (`KismetSystemLibrary.PrintString` (`KismetStringLibrary.Concat_StrStr` (`KismetSystemLibrary.GetDisplayName` OtherActor) "" "Finished")))

(fn `UserConstructionScript`
  (bind (_returnvalue_x _returnvalue_y _returnvalue_z) (`KismetMathLibrary.BreakVector` (`self.K2_GetActorLocation`)))
  (bind (_returnvalue_x_2 _returnvalue_y_2 _returnvalue_z_2) (`KismetMathLibrary.BreakVector` (`self.K2_GetActorLocation`)))
  (bind (_returnvalue_x_3 _returnvalue_y_3 _returnvalue_z_3) (`KismetMathLibrary.BreakVector` (`self.K2_GetActorLocation`)))
  (bind (_returnvalue_x_4 _returnvalue_y_4 _returnvalue_z_4) (`KismetMathLibrary.BreakVector` (`self.K2_GetActorLocation`)))
  (for _index (range (+ (`self.CountLength`) 1))
    (`InstancedStaticMeshComponent.AddInstance` (`self.InstancedStaticMesh`) (`KismetMathLibrary.MakeTransform` (`KismetMathLibrary.MakeVector` (+ (* _index (`self.MeshSize`)) _returnvalue_x) _returnvalue_y _returnvalue_z)) true)
    (for _index_2 (range (+ (`self.CountWidth`) 1))
      (`InstancedStaticMeshComponent.AddInstance` (`self.InstancedStaticMesh`) (`KismetMathLibrary.MakeTransform` (`KismetMathLibrary.MakeVector` _returnvalue_x_2 (+ (* _index_2 (`self.MeshSize`)) _returnvalue_y_2) _returnvalue_z_2)) true))
    (`SceneComponent.K2_SetRelativeLocation` (`self.StartLocation`) (`KismetMathLibrary.MakeVector` _returnvalue_x_3 (+ (* (`self.CountWidth`) (`self.MeshSize`)) _returnvalue_y_3) _returnvalue_z_3) false false))
  (`SceneComponent.K2_SetRelativeLocation` (`self.Loch`) (`KismetMathLibrary.MakeVector` (+ (* (`self.CountLength`) (`self.MeshSize`)) _returnvalue_x_4) _returnvalue_y_4 _returnvalue_z_4) false false))