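; BP_Item is a respawning pickup whose ItemType selects its static mesh in the Construction Script.
; On an authority-side overlap it disables and hides itself, and a three-second timer re-enables and shows it.
; Only the Health type has an effect, healing an overlapping BP_MyTPCharacter; Ammo and Sprintboost only change the mesh.
; Any overlapping actor triggers the cooldown, as the character cast happens afterwards.
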(event `self.StaticMesh.OnComponentBeginOverlap`
  (params (OverlappedComponent :type "PrimitiveComponent Object Reference") (OtherActor :type "Actor Object Reference") (OtherComp :type "PrimitiveComponent Object Reference") (OtherBodyIndex :type Integer) (bFromSweep :type Boolean) (SweepResult :type "HitResult Structure (by ref)"))
  (`/Engine/EditorBlueprintResources/ActorMacros.Switch Has Authority`
    (:`Authority`
      (if (not (`self.Disabled`))
        (set `self.Disabled` true)
        (`KismetSystemLibrary.K2_SetTimerDelegate` (delegate `ResetDisable`) 3.0)
        (`|ExecutionSequence`
          (:`then_0`
            (switch `/Game/Blueprints/E_Item` (`self.ItemType`)
              (:`NewEnumerator1`
                (bind _asbp_my_tpcharacter (cast `/Game/Blueprints/BP_MyTPCharacter` OtherActor))
                (`/Game/Blueprints/BP_MyTPCharacter.AddHealth` _asbp_my_tpcharacter 25.0))))
          (:`then_1`
            (`SceneComponent.SetVisibility` (`self.StaticMesh`) (not (`self.Disabled`)) false :!label _label)))))))

(event `ResetDisable`
  (set `self.Disabled` false)
  (goto _label))

(fn `UserConstructionScript`
  (bind _staticmesh (`self.StaticMesh`))
  (switch `/Game/Blueprints/E_Item` (`self.ItemType`)
    (:`NewEnumerator0`
      (`StaticMeshComponent.SetStaticMesh` _staticmesh "/Game/StarterContent/Shapes/Shape_Cone.Shape_Cone"))
    (:`NewEnumerator1`
      (`StaticMeshComponent.SetStaticMesh` _staticmesh "/Game/StarterContent/Shapes/Shape_Cube.Shape_Cube"))
    (:`NewEnumerator2`
      (`StaticMeshComponent.SetStaticMesh` _staticmesh "/Game/StarterContent/Shapes/Shape_Pipe_90.Shape_Pipe_90"))))